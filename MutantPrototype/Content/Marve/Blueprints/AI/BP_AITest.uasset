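; BP_AITest is a test Blueprint that prints a line of dialogue when one of its body parts is hit.
; Hit events on the Head, Body, LeftFoot, RightFoot and Ass components call a function per region, with both feet sharing one.
; Each function randomly picks one of the first two entries in that region's dialogue array and prints it.
; It contains no AI behaviour or damage logic.
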(event `self.Head.OnComponentHit`
  (params (HitComponent :type "PrimitiveComponent Object Reference") (OtherActor :type "Actor Object Reference") (OtherComp :type "PrimitiveComponent Object Reference") (NormalImpulse :type "Vector Structure") (Hit :type "HitResult Structure (by ref)"))
  (`self.HitHead`))

(event `self.Body.OnComponentHit`
  (params (HitComponent :type "PrimitiveComponent Object Reference") (OtherActor :type "Actor Object Reference") (OtherComp :type "PrimitiveComponent Object Reference") (NormalImpulse :type "Vector Structure") (Hit :type "HitResult Structure (by ref)"))
  (`self.HitBody`))

(event `self.Left Foot.OnComponentHit`
  (params (HitComponent :type "PrimitiveComponent Object Reference") (OtherActor :type "Actor Object Reference") (OtherComp :type "PrimitiveComponent Object Reference") (NormalImpulse :type "Vector Structure") (Hit :type "HitResult Structure (by ref)"))
  (`self.HitFeet`))

(event `self.Right Foot.OnComponentHit`
  (params (HitComponent :type "PrimitiveComponent Object Reference") (OtherActor :type "Actor Object Reference") (OtherComp :type "PrimitiveComponent Object Reference") (NormalImpulse :type "Vector Structure") (Hit :type "HitResult Structure (by ref)"))
  (`self.HitFeet`))

(event `self.Ass.OnComponentHit`
  (params (HitComponent :type "PrimitiveComponent Object Reference") (OtherActor :type "Actor Object Reference") (OtherComp :type "PrimitiveComponent Object Reference") (NormalImpulse :type "Vector Structure") (Hit :type "HitResult Structure (by ref)"))
  (`self.HitAss`))

(fn `HitAss`
  (`KismetSystemLibrary.PrintText` (`|GetArrayItem` (`self.AssDialogue`) (`KismetMathLibrary.RandomInteger` 2))))

(fn `HitBody`
  (`KismetSystemLibrary.PrintText` (`|GetArrayItem` (`self.bodyDialogue`) (`KismetMathLibrary.RandomInteger` 2))))

(fn `HitFeet`
  (`KismetSystemLibrary.PrintText` (`|GetArrayItem` (`self.feetDialogue`) (`KismetMathLibrary.RandomInteger` 2))))

(fn `HitHead`
  (`KismetSystemLibrary.PrintText` (`|GetArrayItem` (`self.headDialogue`) (`KismetMathLibrary.RandomInteger` 2))))

(fn `UserConstructionScript`)