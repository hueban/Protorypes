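; BP_BasicEnemyAi is a basic melee enemy that chases the player and attacks when in range.
; Tick reissues AI MoveTo toward the player; on success, a DoOnce gate plays one of three random attack montages at half speed.
; DamageBox overlap events are on only during the montage, and a DamageDealt flag limits each swing to one hit through the player's ACDamageManager.
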(event `self.ReceiveTick`
  (params (DeltaSeconds :type "Float (single-precision)"))
  (`|AIMoveTo` self (0.0 0.0 0.0) (`GameplayStatics.GetPlayerCharacter` 0) 500.0
    (:`OnSuccess`
      (`/Engine/EditorBlueprintResources/StandardMacros.DoOnce` false :!label _label
        (:`Completed`
          (set `self.DamageDealt` false)
          (`|PlayMontage` (`self.Mesh`) (`|GetArrayItem` (`self.Montage to Play`) (`KismetMathLibrary.RandomIntegerInRange` 0 2)) 0.5
            (:`then`
              (set `PrimitiveComponent.bGenerateOverlapEvents` true (`self.DamageBox`)))
            (:`OnCompleted`
              (set `PrimitiveComponent.bGenerateOverlapEvents` false (`self.DamageBox`))
              (goto _label :!via `Reset`))))))))

(event `self.DamageBox.OnComponentBeginOverlap`
  (params (OverlappedComponent :type "PrimitiveComponent Object Reference") (OtherActor :type "Actor Object Reference") (OtherComp :type "PrimitiveComponent Object Reference") (OtherBodyIndex :type Integer) (bFromSweep :type Boolean) (SweepResult :type "HitResult Structure (by ref)"))
  (if (not (`self.DamageDealt`))
    (bind _asbp_third_person_character (cast `/Game/ThirdPerson/Blueprints/BP_ThirdPersonCharacter` OtherActor))
    (`/Game/CombatSystem/AC_DamageManager.TakeDamage` (`/Game/ThirdPerson/Blueprints/BP_ThirdPersonCharacter.AC_DamageManager` _asbp_third_person_character) 1000.0)
    (set `self.DamageDealt` true)))

(fn `UserConstructionScript`)