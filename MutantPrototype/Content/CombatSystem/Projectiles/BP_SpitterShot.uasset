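; BP_SpitterShot is a combat projectile, apparently fired by a Spitter, that damages what it hits.
; Its Tick chain uses latent Delays to set the Sphere to block all channels shortly after spawn, then destroy the actor about three seconds later.
; On a Sphere hit, it passes Damage to the other actor's AC_DamageManager, if present, and is not destroyed by the impact.
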(event `self.ReceiveTick`
  (params (DeltaSeconds :type "Float (single-precision)"))
  (`KismetSystemLibrary.Delay` 0.05)
  (`PrimitiveComponent.SetCollisionResponseToAllChannels` (`self.Sphere`) "ECR_Block")
  (`KismetSystemLibrary.Delay` 3.0)
  (`self.K2_DestroyActor`))

(event `self.Sphere.OnComponentHit`
  (params (HitComponent :type "PrimitiveComponent Object Reference") (OtherActor :type "Actor Object Reference") (OtherComp :type "PrimitiveComponent Object Reference") (NormalImpulse :type "Vector Structure") (Hit :type "HitResult Structure (by ref)"))
  (bind _output (`|GetArrayItem` (`self.K2_GetComponentsByClass` OtherActor "/Game/CombatSystem/AC_DamageManager.AC_DamageManager_C")))
  (`/Engine/EditorBlueprintResources/StandardMacros.IsValid` _output
    (:`Is Valid`
      (`/Game/CombatSystem/AC_DamageManager.TakeDamage` _output (`self.Damage`)))))

(fn `UserConstructionScript`)