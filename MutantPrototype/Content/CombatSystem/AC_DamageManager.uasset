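; AC_DamageManager is an actor component that tracks health and applies damage to its owning actor in the combat system.
; Health starts at MaxHealth on BeginPlay.
; TakeDamage prints the damage amount on screen, subtracts it from Health, and destroys the owner once Health reaches zero or below.
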(event `self.ReceiveBeginPlay`
  (set `self.Health` (`self.MaxHealth`)))

(fn `TakeDamage`
  (params (DamageDealt :type "Float (double-precision)"))
  (`KismetSystemLibrary.PrintString` (`KismetStringLibrary.Conv_DoubleToString` DamageDealt) true true (struct :`R` 1.0 :`G` 0.036947 :`A` 1.0))
  (set `self.Health` (- (`self.Health`) DamageDealt))
  (if (<= (`self.Health`) 0.0)
    (`Actor.K2_DestroyActor` (`self.GetOwner`))))