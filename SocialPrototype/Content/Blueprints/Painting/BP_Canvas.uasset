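; Paintable canvas actor that lets the third-person character paint while inside its box trigger.
; DrawOnCanvas takes a 2D location and color name, then draws a dynamic brush material, with adjustable size, into that color's own render target.
; Each stroke increments a capped DrawAmount, which ScoreActivity returns rounded as the score.
; ClearCanvas wipes all targets and the count on BeginPlay; an erase material is created but unused here.
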(event `self.ReceiveBeginPlay`
  (bind _returnvalue (`KismetMaterialLibrary.CreateDynamicMaterialInstance` "/Game/Blueprints/Painting/PaintMat.PaintMat"))
  (set `self.PaintMat` _returnvalue)
  (bind _returnvalue_2 (`KismetMaterialLibrary.CreateDynamicMaterialInstance` "/Game/Blueprints/Painting/PaintMatSubtract.PaintMatSubtract"))
  (set `self.ErasePaintMat` _returnvalue_2)
  (`self.ClearCanvas`))

(event `ClearCanvas`
  (`KismetRenderingLibrary.ClearRenderTarget2D` "/Game/Blueprints/Painting/PaintRenderTarget.PaintRenderTarget")
  (`KismetRenderingLibrary.ClearRenderTarget2D` "/Game/Blueprints/Painting/PaintRenderTargetRed.PaintRenderTargetRed")
  (`KismetRenderingLibrary.ClearRenderTarget2D` "/Game/Blueprints/Painting/PaintRenderTargetBlue.PaintRenderTargetBlue")
  (`KismetRenderingLibrary.ClearRenderTarget2D` "/Game/Blueprints/Painting/PaintRenderTargetGreen.PaintRenderTargetGreen")
  (`KismetRenderingLibrary.ClearRenderTarget2D` "/Game/Blueprints/Painting/PaintRenderTargetWhite.PaintRenderTargetWhite")
  (set `self.DrawAmount` 0.0))

(event `DrawOnCanvas`
  (params (CanvasDrawLocation :type "Vector2D Structure") (Color :type String))
  (set `self.DrawLocation` (`KismetMathLibrary.Conv_VectorToLinearColor` (`KismetMathLibrary.Conv_Vector2DToVector` CanvasDrawLocation 0.1)))
  (if (`KismetStringLibrary.EqualEqual_StrStr` Color "Black")
    (`self.PaintBlack`)
    (if (< (`self.DrawAmount`) (`self.DrawAmountMax`)) :!label _label
      (bind _output_get (set `self.DrawAmount` (+ (`self.DrawAmount`) 1.0)))
      (`KismetSystemLibrary.PrintString` (`KismetStringLibrary.Conv_DoubleToString` _output_get)))
    (elif (`KismetStringLibrary.EqualEqual_StrStr` Color "Red")
      (`self.PaintRed`)
      (goto _label)
      (elif (`KismetStringLibrary.EqualEqual_StrStr` Color "Green")
        (`self.PaintGreen`)
        (goto _label)
        (elif (`KismetStringLibrary.EqualEqual_StrStr` Color "Blue")
          (`self.PaintBlue`)
          (goto _label)
          (elif (`KismetStringLibrary.EqualEqual_StrStr` Color "White")
            (`self.PaintWhite`)
            (goto _label)))))))

(event `PaintRed`
  (bind _paintmat (`self.PaintMat`))
  (`MaterialInstanceDynamic.SetVectorParameterValue` _paintmat "DrawLocation" (`self.DrawLocation`))
  (`KismetRenderingLibrary.DrawMaterialToRenderTarget` "/Game/Blueprints/Painting/PaintRenderTargetRed.PaintRenderTargetRed" _paintmat))

(event `DrawSize`
  (params (DrawSize :type "Float (double-precision)"))
  (`MaterialInstanceDynamic.SetScalarParameterValue` (`self.PaintMat`) "Size" DrawSize))

(event `PaintBlack`
  (bind _paintmat (`self.PaintMat`))
  (`MaterialInstanceDynamic.SetVectorParameterValue` _paintmat "DrawLocation" (`self.DrawLocation`))
  (`KismetRenderingLibrary.DrawMaterialToRenderTarget` "/Game/Blueprints/Painting/PaintRenderTarget.PaintRenderTarget" _paintmat))

(event `self.Box.OnComponentBeginOverlap`
  (params (OverlappedComponent :type "PrimitiveComponent Object Reference") (OtherActor :type "Actor Object Reference") (OtherComp :type "PrimitiveComponent Object Reference") (OtherBodyIndex :type Integer) (bFromSweep :type Boolean) (SweepResult :type "HitResult Structure (by ref)"))
  (bind _asbp_third_person_character (cast `/Game/ThirdPerson/Blueprints/BP_ThirdPersonCharacter` OtherActor))
  (set `/Game/ThirdPerson/Blueprints/BP_ThirdPersonCharacter.CanPaint` true _asbp_third_person_character))

(event `PaintBlue`
  (bind _paintmat (`self.PaintMat`))
  (`MaterialInstanceDynamic.SetVectorParameterValue` _paintmat "DrawLocation" (`self.DrawLocation`))
  (`KismetRenderingLibrary.DrawMaterialToRenderTarget` "/Game/Blueprints/Painting/PaintRenderTargetBlue.PaintRenderTargetBlue" _paintmat))

(event `self.Box.OnComponentEndOverlap`
  (params (OverlappedComponent :type "PrimitiveComponent Object Reference") (OtherActor :type "Actor Object Reference") (OtherComp :type "PrimitiveComponent Object Reference") (OtherBodyIndex :type Integer))
  (bind _asbp_third_person_character (cast `/Game/ThirdPerson/Blueprints/BP_ThirdPersonCharacter` OtherActor))
  (set `/Game/ThirdPerson/Blueprints/BP_ThirdPersonCharacter.CanPaint` false _asbp_third_person_character))

(event `PaintGreen`
  (bind _paintmat (`self.PaintMat`))
  (`MaterialInstanceDynamic.SetVectorParameterValue` _paintmat "DrawLocation" (`self.DrawLocation`))
  (`KismetRenderingLibrary.DrawMaterialToRenderTarget` "/Game/Blueprints/Painting/PaintRenderTargetGreen.PaintRenderTargetGreen" _paintmat))

(event `PaintWhite`
  (bind _paintmat (`self.PaintMat`))
  (`MaterialInstanceDynamic.SetVectorParameterValue` _paintmat "DrawLocation" (`self.DrawLocation`))
  (`KismetRenderingLibrary.DrawMaterialToRenderTarget` "/Game/Blueprints/Painting/PaintRenderTargetWhite.PaintRenderTargetWhite" _paintmat))

(fn `ScoreActivity`
  (returns (Score :type "Float (double-precision)"))
  (return (`KismetMathLibrary.Conv_IntToDouble` (`KismetMathLibrary.Round` (`self.DrawAmount`)))))

(fn `UserConstructionScript`)