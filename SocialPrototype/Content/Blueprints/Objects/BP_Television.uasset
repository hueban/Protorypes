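; BP_Television is an interactable TV that attracts pedestrians to watch it and lets the player send them away.
; Pedestrians entering Box whose UI widget personality matches the TV's take the next of six watch locations, up to MaxPeople.
; While the player character is inside Box1, TriggerInteract makes pedestrians in Box end their activity, resume random roaming and clear their Bored flag.
; PeopleWatching only increments and is never reset here.
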(event `self.ReceiveBeginPlay`
  (set `self.Locations` (`|MakeArray` (`self.WatchLocation1`) (`self.WatchLocation2`) (`self.WatchLocation3`) (`self.WatchLocation4`) (`self.WatchLocation5`) (`self.WatchLocation6`))))

(event `self.Box.OnComponentBeginOverlap`
  (params (OverlappedComponent :type "PrimitiveComponent Object Reference") (OtherActor :type "Actor Object Reference") (OtherComp :type "PrimitiveComponent Object Reference") (OtherBodyIndex :type Integer) (bFromSweep :type Boolean) (SweepResult :type "HitResult Structure (by ref)"))
  (if (< (`self.PeopleWatching`) (`self.MaxPeople`))
    (bind _asbp_pedestrian (cast `/Game/ThirdPerson/Marve/Blueprints/AI/BP_Pedestrian` OtherActor))
    (bind _asbpw_pedestrian_ui (cast `/Game/ThirdPerson/Marve/Blueprints/UI/BPW_PedestrianUI` (`WidgetComponent.GetWidget` (`/Game/ThirdPerson/Marve/Blueprints/AI/BP_Pedestrian.Widget` _asbp_pedestrian))))
    (if (`KismetTextLibrary.EqualEqual_TextText` (`/Game/ThirdPerson/Marve/Blueprints/UI/BPW_PedestrianUI.GetPersonality` _asbpw_pedestrian_ui) (`self.Personallity`))
      (bind _output_get (set `self.PeopleWatching` (+ (`self.PeopleWatching`) 1.0)))
      (bind _returnvalue (- (`KismetMathLibrary.FTrunc` _output_get) 1))
      (if (`KismetArrayLibrary.Array_IsValidIndex` (`self.Locations`) _returnvalue)
        (`/Game/ThirdPerson/Marve/Blueprints/AI/BP_Pedestrian.WatchTV` _asbp_pedestrian (`SceneComponent.K2_GetComponentToWorld` (`|GetArrayItem` (`self.Locations`) _returnvalue)))))))

(event `self.Box1.OnComponentBeginOverlap`
  (params (OverlappedComponent :type "PrimitiveComponent Object Reference") (OtherActor :type "Actor Object Reference") (OtherComp :type "PrimitiveComponent Object Reference") (OtherBodyIndex :type Integer) (bFromSweep :type Boolean) (SweepResult :type "HitResult Structure (by ref)"))
  (cast `/Game/ThirdPerson/Blueprints/BP_ThirdPersonCharacter` OtherActor)
  (set `self.CanTurnOff` true))

(event `/Game/ThirdPerson/Blueprints/Interact.TriggerInteract`
  (if (`self.CanTurnOff`)
    (for _array_element (`PrimitiveComponent.GetOverlappingActors` (`self.Box`) "/Game/ThirdPerson/Marve/Blueprints/AI/BP_Pedestrian.BP_Pedestrian_C")
      (bind _asbp_pedestrian (cast `/Game/ThirdPerson/Marve/Blueprints/AI/BP_Pedestrian` _array_element))
      (set `/Game/ThirdPerson/Marve/Blueprints/AI/BP_Pedestrian.DoingActivity` false _asbp_pedestrian)
      (`/Game/ThirdPerson/Marve/Blueprints/AI/BP_Pedestrian.Random Roam` _asbp_pedestrian)
      (set `/Game/ThirdPerson/Marve/Blueprints/AI/AC_NpcDialogueManager.Bored` false (`/Game/ThirdPerson/Marve/Blueprints/AI/BP_Pedestrian.AC_NpcDialogueManager` _asbp_pedestrian)))))

(event `self.Box1.OnComponentEndOverlap`
  (params (OverlappedComponent :type "PrimitiveComponent Object Reference") (OtherActor :type "Actor Object Reference") (OtherComp :type "PrimitiveComponent Object Reference") (OtherBodyIndex :type Integer))
  (cast `/Game/ThirdPerson/Blueprints/BP_ThirdPersonCharacter` OtherActor)
  (set `self.CanTurnOff` false))

(fn `UserConstructionScript`)