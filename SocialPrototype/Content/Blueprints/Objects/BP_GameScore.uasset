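; BP_GameScore is a two-team scoreboard object that also reports itself as a scored activity.
; AddScore increments the given team's component of Scores and updates Score1 or Score2 text, zeroing the other team's value without refreshing its display.
; ScoreActivity returns a random score scaled from Team 1's count, along with the required personality, required skill and interest values.
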(event `self.ReceiveTick`
  (params (DeltaSeconds :type "Float (single-precision)")))

(event `AddScore`
  (params (Team :type Integer))
  (bind (_scores_x _scores_y) (`KismetMathLibrary.BreakVector2D` (`self.Scores`)))
  (bind _scores_x_2 (`KismetMathLibrary.BreakVector2D` (`self.Scores`)))
  (if (== Team 1)
    (bind _output_get (set `self.Scores` (`KismetMathLibrary.MakeVector2D` (+ _scores_x_2 1.0))))
    (`TextRenderComponent.K2_SetText` (`self.Score1`) (`KismetTextLibrary.Conv_DoubleToText` (`KismetMathLibrary.BreakVector2D` _output_get) "HalfToEven"))
    (elif (== Team 2)
      (bind _output_get_2 (set `self.Scores` (`KismetMathLibrary.MakeVector2D` 0.0 (+ _scores_y 1.0))))
      (`TextRenderComponent.K2_SetText` (`self.Score2`) (`KismetTextLibrary.Conv_DoubleToText` (`.Y` (`KismetMathLibrary.BreakVector2D` _output_get_2)) "HalfToEven")))))

(fn `ScoreActivity`
  (returns (Score :type "Float (double-precision)") (Personallity :type Text) (Skill :type Text) (Interest :type Text))
  (bind _scores_x (`KismetMathLibrary.BreakVector2D` (`self.Scores`)))
  (return (`KismetMathLibrary.RandomFloatInRange` (* _scores_x 100.0) (* _scores_x 1000.0)) (`self.PersonalityRequired`) (`self.SkillRequired`) (`self.Interest`)))

(fn `UserConstructionScript`)